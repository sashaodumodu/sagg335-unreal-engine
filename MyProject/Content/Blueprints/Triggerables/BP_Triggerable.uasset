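; BP_Triggerable is a trigger actor that reacts when other actors enter or leave its Trigger component.
; Begin and end overlap events pass the other actor through a ClassIsChildOf check, then forward it to the custom Overlapped and UnOverlapped events.
; Those two events only print the actor's display name, serving as simple debug responses.
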(event OnComponentBeginOverlap(Trigger)
  (params (OverlappedComponent :type Primitive%20Component%20Object%20Reference) (OtherActor :type Actor%20Object%20Reference) (OtherComp :type Primitive%20Component%20Object%20Reference) (OtherBodyIndex :type Integer) (bFromSweep :type Boolean) (SweepResult :type Hit%20Result%20Structure%20%28by%20ref%29))
  (if (Utilities|ClassIsChildOf (Utilities|GetClass OtherActor) 0)
    (CallFunction|Overlapped OtherActor)))

(event OnComponentEndOverlap(Trigger)
  (params (OverlappedComponent :type Primitive%20Component%20Object%20Reference) (OtherActor :type Actor%20Object%20Reference) (OtherComp :type Primitive%20Component%20Object%20Reference) (OtherBodyIndex :type Integer))
  (if (Utilities|ClassIsChildOf (Utilities|GetClass OtherActor) 0)
    (CallFunction|UnOverlapped OtherActor)))

(event Custom|Overlapped
  (params (Other%20Actor :type Object%20Object%20Reference))
  (Development|PrintString (Utilities|GetDisplayName Other%20Actor)))

(event Custom|UnOverlapped
  (params (Other%20Actor :type Object%20Object%20Reference))
  (Development|PrintString (Utilities|GetDisplayName Other%20Actor)))

(event EventBeginPlay)

(event Collision|EventActorBeginOverlap
  (params (OtherActor :type Actor%20Object%20Reference)))

(event EventTick
  (params (DeltaSeconds :type Float%20%28single-precision%29)))

(fn ConstructionScript)